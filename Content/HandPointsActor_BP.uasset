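; Marker actor that follows one tracked mixed-reality hand joint, copying its transform from motion controller hand data each Tick.
; For the palm and fingertips, a spawned TextRenderActor shows location and rotation as debug text.
; Each Tick it compares enabled axes against the pawn's OpenHandPositions entry within tolerances, computing whether the joint is in pose.
; Overlapping an InteractiveActor_BP plays timelines that change its point light's intensity.
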(event `self.ReceiveBeginPlay`
  (`PrimitiveComponent.SetMaterial` (`self.StaticMesh`) 0 "/Game/Materials/Transparency_Material.Transparency_Material")
  (bind _outactors (`GameplayStatics.GetAllActorsOfClass` "/Game/MRPawn_BP.MRPawn_BP_C"))
  (set `self.MRPawn` (`|GetArrayItem` _outactors))
  (if (or (`|EnumEquality` (`self.Bone`) "Palm") (`|EnumEquality` (`self.Bone`) "ThumbTip") (`|EnumEquality` (`self.Bone`) "IndexTip") (`|EnumEquality` (`self.Bone`) "MiddleTip") (`|EnumEquality` (`self.Bone`) "RingTip") (`|EnumEquality` (`self.Bone`) "LittleTip"))
    (bind _returnvalue (`|SpawnActorFromClass` "/Script/Engine.TextRenderActor" (`KismetMathLibrary.MakeTransform` (0.0 0.0 0.0)) "AlwaysSpawn" "OverrideRootScale" self null))
    (set `self.Hand Text` _returnvalue)
    (`PrimitiveComponent.SetMaterial` (`TextRenderActor.TextRender` _returnvalue) 0 "/Game/Materials/Transparency_Material.Transparency_Material")))

(event `self.ReceiveTick`
  (params (DeltaSeconds :type "Float (single-precision)"))
  (`self.Update Node Position`)
  (`self.SetHandText`)
  (`self.Test Node Position` (`/Game/MRPawn_BP.Open Hand Positions` (`self.MRPawn`))))

(event `self.StaticMesh.OnComponentBeginOverlap`
  (params (OverlappedComponent :type "PrimitiveComponent Object Reference") (OtherActor :type "Actor Object Reference") (OtherComp :type "PrimitiveComponent Object Reference") (OtherBodyIndex :type Integer) (bFromSweep :type Boolean) (SweepResult :type "HitResult Structure (by ref)"))
  (bind _brightnessmultiplier (`self.BrightnessMultiplier`))
  (bind _pointlight (`self.PointLight`))
  (cast `/Game/InteractiveActor_BP` OtherActor)
  (`|ExecutionSequence`
    (:`then_0`
      (bind (_direction _lightbrightnessfloattrack) (`Timeline|Timeline_0` :!via `Stop` :!label _label)
        (:`Update`
          (`LightComponent.SetIntensity` _pointlight (* _lightbrightnessfloattrack _brightnessmultiplier)))))
    (:`then_1`
      (bind (_direction_2 _lightbrightnessfloattrack_2) (`Timeline|Timeline_1` :!label _label_2)
        (:`Update`
          (`LightComponent.SetIntensity` _pointlight (* _lightbrightnessfloattrack_2 _brightnessmultiplier)))))))

(event `self.StaticMesh.OnComponentEndOverlap`
  (params (OverlappedComponent :type "PrimitiveComponent Object Reference") (OtherActor :type "Actor Object Reference") (OtherComp :type "PrimitiveComponent Object Reference") (OtherBodyIndex :type Integer))
  (cast `/Game/InteractiveActor_BP` OtherActor)
  (`|ExecutionSequence`
    (:`then_0`
      (goto _label_2 :!via `Stop`))
    (:`then_1`
      (goto _label))))

(fn `SetHandText`
  (bind _hand_text (`self.Hand Text`))
  (bind _location (.location (`self.GetTransform` self)))
  (`/Engine/EditorBlueprintResources/StandardMacros.IsValid` self
    (:`Is Valid`
      (`/Engine/EditorBlueprintResources/StandardMacros.IsValid` _hand_text
        (:`Is Valid`
          (`self.K2_SetActorTransform` _hand_text (`KismetMathLibrary.MakeTransform` (+ (* _location (1.0 1.0 1.0)) (10.0 5.0 5.0)) (struct :`Yaw` 180.0) (`KismetMathLibrary.Conv_DoubleToVector` 0.05)) false false)
          (`TextRenderComponent.K2_SetText` (`TextRenderActor.TextRender` _hand_text) (`KismetTextLibrary.Conv_StringToText` (`KismetStringLibrary.Concat_StrStr` "L: X=" (`KismetStringLibrary.Conv_IntToString` (`KismetMathLibrary.Conv_Int64ToInt` (`KismetMathLibrary.Round64` (.x _location)))) "   Y=" (`KismetStringLibrary.Conv_IntToString` (`KismetMathLibrary.Conv_Int64ToInt` (`KismetMathLibrary.Round64` (.y _location)))) "   Z=" (`KismetStringLibrary.Conv_IntToString` (`KismetMathLibrary.Conv_Int64ToInt` (`KismetMathLibrary.Round64` (.z _location)))) " \n" (`KismetStringLibrary.Concat_StrStr` "R: X=" (`KismetStringLibrary.Conv_IntToString` (`KismetMathLibrary.Conv_Int64ToInt` (`KismetMathLibrary.Round64` (.roll (`self.K2_GetActorRotation` self))))) "   Y=" (`KismetStringLibrary.Conv_IntToString` (`KismetMathLibrary.Conv_Int64ToInt` (`KismetMathLibrary.Round64` (.pitch (`self.K2_GetActorRotation` self))))) "   Z=" (`KismetStringLibrary.Conv_IntToString` (`KismetMathLibrary.Conv_Int64ToInt` (`KismetMathLibrary.Round64` (.yaw (`self.K2_GetActorRotation` self)))))))))
          (return))))))

(fn `Test Node Position`
  (params (`Hand Piont Positions` :type "Map of EHandKeypoint Enum to HandPointPosition Structure (by ref)"))
  (returns (ReturnValue :type Boolean))
  (bind (_value _returnvalue) (`BlueprintMapLibrary.Map_Find` `Hand Piont Positions` (`self.Bone`)))
  (bind (_isinposition _activematerial _locationpoints _locationerrortolerance _rotationpoints _rotatorerrortolerance) (break `HandPointPosition` _value))
  (bind (_usex _x _usey _y _usez _z) (break `BoolandVectorPair` _locationpoints))
  (bind (_usex_2 _x_2 _usey_2 _y_2 _usez_2 _z_2) (break `BoolandVectorPair` _rotationpoints))
  (bind _returnvalue_2 (and (`KismetMathLibrary.NearlyEqual_FloatFloat` _x (.x (.location (`self.GetTransform`))) _locationerrortolerance) _usex))
  (bind _returnvalue_3 (and (`KismetMathLibrary.NearlyEqual_FloatFloat` _y (.y (.location (`self.GetTransform`))) _locationerrortolerance) _usey))
  (bind _returnvalue_4 (and (`KismetMathLibrary.NearlyEqual_FloatFloat` _z (.z (.location (`self.GetTransform`))) _locationerrortolerance) _usez))
  (bind _returnvalue_5 (and (`KismetMathLibrary.NearlyEqual_FloatFloat` (.roll (`self.K2_GetActorRotation`)) _x_2 _rotatorerrortolerance) _usex_2))
  (bind _returnvalue_6 (and (`KismetMathLibrary.NearlyEqual_FloatFloat` (.pitch (`self.K2_GetActorRotation`)) _y_2 _rotatorerrortolerance) _usey_2))
  (bind _returnvalue_7 (and (`KismetMathLibrary.NearlyEqual_FloatFloat` (.yaw (`self.K2_GetActorRotation`)) _z_2 _rotatorerrortolerance) _usez_2))
  (bind _returnvalue_8 (and (== (+ (`KismetMathLibrary.Conv_BoolToInt` _usez_2) (`KismetMathLibrary.Conv_BoolToInt` _usey_2) (`KismetMathLibrary.Conv_BoolToInt` _usex) (`KismetMathLibrary.Conv_BoolToInt` _usez) (`KismetMathLibrary.Conv_BoolToInt` _usey) (`KismetMathLibrary.Conv_BoolToInt` _usex_2)) (+ (`KismetMathLibrary.Conv_BoolToInt` _returnvalue_2) (`KismetMathLibrary.Conv_BoolToInt` _returnvalue_3) (`KismetMathLibrary.Conv_BoolToInt` _returnvalue_4) (`KismetMathLibrary.Conv_BoolToInt` _returnvalue_5) (`KismetMathLibrary.Conv_BoolToInt` _returnvalue_6) (`KismetMathLibrary.Conv_BoolToInt` _returnvalue_7))) (or _returnvalue_2 _returnvalue_3 _returnvalue_4 _returnvalue_5 _returnvalue_6 _returnvalue_7)))
  (if _returnvalue
    (if _returnvalue_8
      _
      (else
        _))
    (setmembers `HandPointPosition` :`StructRef` _value :`IsInPosition` _returnvalue_8)
    (return _returnvalue_8)
    (else
      (return false))))

(fn `Update Node Position`
  (bind _returnvalue (`KismetMathLibrary.Conv_ByteToInt` (`self.Bone`)))
  (bind _motioncontrollerdata (`HeadMountedDisplayFunctionLibrary.GetMotionControllerData` null (`self.Hand`)))
  (bind (_bvalid _devicename _applicationinstanceid _devicevisualtype _handindex _trackingstatus _gripposition _griprotation _aimposition _aimrotation _handkeypositions _handkeyrotations _handkeyradii) (break `XRMotionControllerData` _motioncontrollerdata))
  (if (and _bvalid (`|EnumEquality` _devicevisualtype "Hand"))
    (`self.K2_SetActorTransform` (`KismetMathLibrary.MakeTransform` (`|GetArrayItem` _handkeypositions _returnvalue) (`KismetMathLibrary.Quat_Rotator` (`|GetArrayItem` _handkeyrotations _returnvalue)) (`KismetMathLibrary.Conv_DoubleToVector` (`self.HandPointScale`))))))

(fn `UserConstructionScript`)