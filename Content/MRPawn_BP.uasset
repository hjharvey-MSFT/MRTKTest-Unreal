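; Mixed reality pawn that adds hand-tracked gestures for conjuring objects and summoning interactive actors.
; BeginPlay spawns the MR container, UXT hand interactors and an actor per keypoint of each hand, mapped by keypoint.
; Pressing matching keypoints together starts a Niagara effect and timer, apparently arming an object spawn at the palms' midpoint upon separation.
; Otherwise, an open-hand pose traces from each palm along eye gaze, pulling any hit InteractiveActor toward it.
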(event `self.ReceiveBeginPlay`
  (bind _returnvalue (`KismetMathLibrary.Conv_VectorToTransform` (0.0 0.0 0.0)))
  (`|SpawnActorFromClass` "/Game/MRContainerActor_BP.MRContainerActor_BP_C" _returnvalue "Undefined" "OverrideRootScale" self null)
  (`|SpawnActorFromClass` "/Script/UXTools.UxtHandInteractionActor" _returnvalue "Undefined" "OverrideRootScale" self false "Left" null)
  (`|SpawnActorFromClass` "/Script/UXTools.UxtHandInteractionActor" _returnvalue "Undefined" "OverrideRootScale" self false "Right" null)
  (`MicrosoftOpenXRFunctionLibrary.SetUseHandMesh` "EnabledTrackingGeometry")
  (`self.SpawnHands`))

(event `self.ReceiveTick`
  (params (DeltaSeconds :type "Float (single-precision)"))
  (bind _value (`BlueprintMapLibrary.Map_Find` (`self.RightHandPointsMap`) "Palm"))
  (bind _value_2 (`BlueprintMapLibrary.Map_Find` (`self.LeftHandPointsMap`) "Palm"))
  (bind _returnvalue (+ (/ (`self.K2_GetActorLocation` _value_2) 2.0) (/ (`self.K2_GetActorLocation` _value) 2.0)))
  (if (`self.Hands Are Touching`)
    (`SceneComponent.K2_SetWorldLocation` (`self.SummonParticalEffect`) _returnvalue false true)
    (if (>= (`self.GetDistanceTo` _value_2 _value) 20.0)
      (set `self.Hands Are Touching` false)
      (`ActorComponent.K2_DestroyComponent` (`self.SummonParticalEffect`))
      (if (`self.Should Spawn Object`)
        (set `self.Should Spawn Object` false)
        (`|SpawnActorFromClass` "/Game/InteractiveActor_BP.InteractiveActor_BP_C" (`KismetMathLibrary.MakeTransform` _returnvalue (struct) (0.05 0.05 0.05)) "Undefined" "OverrideRootScale" null null)))
    (else
      (`self.Point close to point`)
      (`self.Check Hand Positions` (`self.LeftHandPointsMap`))
      (`self.Check Hand Positions` (`self.RightHandPointsMap`)))))

(fn `Check Hand Positions`
  (params (TargetMap :type "Map of EHandKeypoint Enum to /Game/HandPointsActor_BP Object Reference (by ref)"))
  (locals (`Finger Location Tolerance` :type "Float (double-precision)" :default 20.0))
  (bind _returnvalue (`self.K2_GetActorLocation` (`BlueprintMapLibrary.Map_Find` TargetMap (enumliteral `EHandKeypoint` "Palm"))))
  (bind _is_open_hand (`self.Hand Open Position`))
  (if _is_open_hand
    (bind (_outgazedata _returnvalue_2) (`EyeTrackerFunctionLibrary.GetGazeData`))
    (if _returnvalue_2
      (bind _values (`BlueprintMapLibrary.Map_Values` TargetMap))
      (bind (_outhit _returnvalue_3) (`KismetSystemLibrary.LineTraceSingle` _returnvalue (+ _returnvalue (* (`.GazeDirection` (break `EyeTrackerGazeData` _outgazedata)) 1000)) "TraceTypeQuery1" false _values "ForOneFrame"))
      (if _returnvalue_3
        (bind (_bblockinghit _binitialoverlap _time _distance _location _impactpoint _normal _impactnormal _physmat _hitactor) (`GameplayStatics.BreakHitResult` _outhit))
        (`KismetSystemLibrary.PrintString` (`KismetSystemLibrary.GetDisplayName` _hitactor))
        (bind _asinteractive_actor_bp (cast `/Game/InteractiveActor_BP` _hitactor)
          (:`then`
            (`self.K2_SetActorLocation` _asinteractive_actor_bp (`KismetMathLibrary.VInterpTo` (`self.K2_GetActorLocation` _asinteractive_actor_bp) (+ _returnvalue (10.0 0.0 0.0)) 1.0 0.05) false false))
          (:`CastFailed`
            _)))))
  (return))

(fn `Hand Open Position`
  (returns (`Is Open Hand` :type Boolean))
  (locals (`Finger Location Tol` :type Boolean))
  (bind _values (`BlueprintMapLibrary.Map_Values` (`self.Open Hand Positions`)))
  (for _array_element _values
    (if (not (`.IsInPosition` (break `HandPointPosition` _array_element)))
      (return false)))
  (return true))

(fn `Point close to point`
  (bind _lefthandpointsmap (`self.LeftHandPointsMap`))
  (for _index (range (`BlueprintMapLibrary.Map_Length` _lefthandpointsmap))
    (bind _returnvalue (cast `EHandKeypoint` (`KismetMathLibrary.Conv_IntToByte` _index)))
    (bind (_value _returnvalue_2) (`BlueprintMapLibrary.Map_Find` _lefthandpointsmap _returnvalue))
    (bind (_value_2 _returnvalue_3) (`BlueprintMapLibrary.Map_Find` (`self.RightHandPointsMap`) _returnvalue))
    (if (and _returnvalue_2 _returnvalue_3)
      (if (not (== (`self.K2_GetActorLocation` _value) (`self.K2_GetActorLocation` _value_2) :`ErrorTolerance` 5.0))
        (return))
      (else
        (return))))
  (if (not (`self.Hands Are Touching`))
    (bind _returnvalue_4 (`AddComponent|NODE_AddNiagaraComponent-0` :`RelativeTransform` (`KismetMathLibrary.MakeTransform` (+ (/ (`self.K2_GetActorLocation` (`BlueprintMapLibrary.Map_Find` (`self.LeftHandPointsMap`) "Palm")) 2.0) (/ (`self.K2_GetActorLocation` (`BlueprintMapLibrary.Map_Find` (`self.RightHandPointsMap`) "Palm")) 2.0)) (struct) (0.05 0.05 0.05))))
    (set `self.SummonParticalEffect` _returnvalue_4)
    (set `self.Hands Are Touching` true)
    (`KismetSystemLibrary.K2_SetTimerDelegate` (`|CreateDelegate` :!event `Spawn Object Test`) 2.0)))

(fn `Spawn Object Test`
  (if (`self.Hands Are Touching`)
    (set `self.Should Spawn Object` true)))

(fn `SpawnHandPoints`
  (params (HandPointTransform :type "Transform Structure") (HandPontIndex :type Integer) (Hand :type "EControllerHand Enum" :default "Left") (TargetMap :type "Map of EHandKeypoint Enum to /Game/HandPointsActor_BP Object Reference (by ref)"))
  (bind _returnvalue (cast `EHandKeypoint` (`KismetMathLibrary.Conv_IntToByte` HandPontIndex)))
  (bind _returnvalue_2 (`|SpawnActorFromClass` "/Game/HandPointsActor_BP.HandPointsActor_BP_C" HandPointTransform "Undefined" "OverrideRootScale" self Hand _returnvalue null))
  (`BlueprintMapLibrary.Map_Add` TargetMap _returnvalue _returnvalue_2))

(fn `SpawnHands`
  (bind _returnvalue (`KismetMathLibrary.MakeTransform` (0.0 0.0 0.0)))
  (bind _enumvalue (foreach `EHandKeypoint` false)
    (:`LoopBody`
      (bind _returnvalue_2 (`KismetMathLibrary.Conv_ByteToInt` _enumvalue))
      (`self.SpawnHandPoints` _returnvalue _returnvalue_2 "Left" (`self.LeftHandPointsMap`))
      (`self.SpawnHandPoints` _returnvalue _returnvalue_2 "Right" (`self.RightHandPointsMap`)))))

(fn `UserConstructionScript`)