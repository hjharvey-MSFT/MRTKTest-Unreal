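; Physics cube actor for mixed reality that the player can grab with tracked hands.
; Overlaps with HandPointsActor keypoints fill per-hand bone lists, and a hand holds it when a thumb point and another finger point both overlap.
; Holding disables physics and collision and attaches the actor to that palm on MRPawn; release restores default physics and damping.
; While physics collision is on, a short downward trace each tick enables gravity only above a surface.
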(event `self.ReceiveBeginPlay`
  (bind _returnvalue (`GameplayStatics.GetActorOfClass` "/Script/MRTKTest.MRPawn"))
  (bind _asmrpawn_bp (cast `/Game/MRPawn_BP` _returnvalue))
  (set `self.MRPawn` _asmrpawn_bp)
  (`self.Set Default Settings`))

(event `self.OverlapCube.OnComponentBeginOverlap`
  (params (OverlappedComponent :type "PrimitiveComponent Object Reference") (OtherActor :type "Actor Object Reference") (OtherComp :type "PrimitiveComponent Object Reference") (OtherBodyIndex :type Integer) (bFromSweep :type Boolean) (SweepResult :type "HitResult Structure (by ref)"))
  (bind _ashand_points_actor_bp (cast `/Game/HandPointsActor_BP` OtherActor))
  (if (`|EnumEquality` (`/Game/HandPointsActor_BP.Hand` _ashand_points_actor_bp) "Left")
    (`KismetArrayLibrary.Array_AddUnique` (`self.Left Hand Overlapping Points`) (`/Game/HandPointsActor_BP.Bone` _ashand_points_actor_bp))
    (else
      (`KismetArrayLibrary.Array_AddUnique` (`self.Right Hand Overlapping Points`) (`/Game/HandPointsActor_BP.Bone` _ashand_points_actor_bp))))
  (`self.Handle Holding`))

(event `self.OverlapCube.OnComponentEndOverlap`
  (params (OverlappedComponent :type "PrimitiveComponent Object Reference") (OtherActor :type "Actor Object Reference") (OtherComp :type "PrimitiveComponent Object Reference") (OtherBodyIndex :type Integer))
  (bind _ashand_points_actor_bp (cast `/Game/HandPointsActor_BP` OtherActor))
  (if (`|EnumEquality` (`/Game/HandPointsActor_BP.Hand` _ashand_points_actor_bp) "Left")
    (`KismetArrayLibrary.Array_RemoveItem` (`self.Left Hand Overlapping Points`) (`/Game/HandPointsActor_BP.Bone` _ashand_points_actor_bp))
    (else
      (`KismetArrayLibrary.Array_RemoveItem` (`self.Right Hand Overlapping Points`) (`/Game/HandPointsActor_BP.Bone` _ashand_points_actor_bp))))
  (`self.Handle Holding`))

(event `self.ReceiveTick`
  (params (DeltaSeconds :type "Float (single-precision)"))
  (bind _cube (`self.Cube`))
  (bind _returnvalue (`SceneComponent.K2_GetComponentLocation` (`self.Cube`)))
  (if (`PrimitiveComponent.K2_IsPhysicsCollisionEnabled` _cube)
    (bind (_outhit _returnvalue_2) (`KismetSystemLibrary.LineTraceSingle` _returnvalue (+ _returnvalue (0.0 0.0 -50.0)) "TraceTypeQuery1"))
    (`PrimitiveComponent.SetEnableGravity` _cube _returnvalue_2)))

(fn `Attach to Palm`
  (params (Condition :type Boolean) (TargetMap :type "Map of EHandKeypoint Enum to /Game/HandPointsActor_BP Object Reference (by ref)"))
  (if Condition
    (`self.K2_AttachToActor` (`BlueprintMapLibrary.Map_Find` TargetMap "Palm") "None" "KeepWorld" "KeepWorld" "KeepWorld" false)))

(fn `Check Hand Holding`
  (params (`Overlapping Points` :type "Array of EHandKeypoint Enum"))
  (returns (`Is Holding` :type Boolean))
  (return (and (or (`KismetArrayLibrary.Array_Contains` `Overlapping Points` (enumliteral `EHandKeypoint` "ThumbMetacarpal")) (`KismetArrayLibrary.Array_Contains` `Overlapping Points` (enumliteral `EHandKeypoint` "ThumbProximal")) (`KismetArrayLibrary.Array_Contains` `Overlapping Points` (enumliteral `EHandKeypoint` "ThumbDistal")) (`KismetArrayLibrary.Array_Contains` `Overlapping Points` (enumliteral `EHandKeypoint` "ThumbTip"))) (or (`KismetArrayLibrary.Array_Contains` `Overlapping Points` (enumliteral `EHandKeypoint` "IndexMetacarpal")) (`KismetArrayLibrary.Array_Contains` `Overlapping Points` (enumliteral `EHandKeypoint` "IndexProximal")) (`KismetArrayLibrary.Array_Contains` `Overlapping Points` (enumliteral `EHandKeypoint` "IndexIntermediate")) (`KismetArrayLibrary.Array_Contains` `Overlapping Points` (enumliteral `EHandKeypoint` "IndexDistal")) (`KismetArrayLibrary.Array_Contains` `Overlapping Points` (enumliteral `EHandKeypoint` "IndexTip")) (`KismetArrayLibrary.Array_Contains` `Overlapping Points` (enumliteral `EHandKeypoint` "RingMetacarpal")) (`KismetArrayLibrary.Array_Contains` `Overlapping Points` (enumliteral `EHandKeypoint` "RingProximal")) (`KismetArrayLibrary.Array_Contains` `Overlapping Points` (enumliteral `EHandKeypoint` "MiddleIntermediate")) (`KismetArrayLibrary.Array_Contains` `Overlapping Points` (enumliteral `EHandKeypoint` "MiddleDistal")) (`KismetArrayLibrary.Array_Contains` `Overlapping Points` (enumliteral `EHandKeypoint` "MiddleTip")) (`KismetArrayLibrary.Array_Contains` `Overlapping Points` (enumliteral `EHandKeypoint` "RingMetacarpal")) (`KismetArrayLibrary.Array_Contains` `Overlapping Points` (enumliteral `EHandKeypoint` "RingProximal")) (`KismetArrayLibrary.Array_Contains` `Overlapping Points` (enumliteral `EHandKeypoint` "RingIntermediate")) (`KismetArrayLibrary.Array_Contains` `Overlapping Points` (enumliteral `EHandKeypoint` "RingDistal")) (`KismetArrayLibrary.Array_Contains` `Overlapping Points` (enumliteral `EHandKeypoint` "RingTip")) (`KismetArrayLibrary.Array_Contains` `Overlapping Points` (enumliteral `EHandKeypoint` "LittleMetacarpal")) (`KismetArrayLibrary.Array_Contains` `Overlapping Points` (enumliteral `EHandKeypoint` "LittleProximal")) (`KismetArrayLibrary.Array_Contains` `Overlapping Points` (enumliteral `EHandKeypoint` "LittleIntermediate")) (`KismetArrayLibrary.Array_Contains` `Overlapping Points` (enumliteral `EHandKeypoint` "LittleDistal")) (`KismetArrayLibrary.Array_Contains` `Overlapping Points` (enumliteral `EHandKeypoint` "LittleTip"))))))

(fn `Handle Holding`
  (bind _mrpawn (`self.MRPawn`))
  (bind _is_holding (`self.Check Hand Holding` (`self.Left Hand Overlapping Points`)))
  (bind _is_holding_2 (`self.Check Hand Holding` (`self.Right Hand Overlapping Points`)))
  (bind _output_get (set `self.Is Held` (or _is_holding _is_holding_2)))
  (if _output_get
    (if _is_holding
      (if _is_holding_2
        (if _is_holding_2 :!label _label
          (`self.set Held Settings` :!label _label_2)
          (`self.Attach to Palm` _is_holding (`/Game/MRPawn_BP.LeftHandPointsMap` _mrpawn))
          (`self.Attach to Palm` _is_holding_2 (`/Game/MRPawn_BP.RightHandPointsMap` _mrpawn))
          (else
            (`self.Set Default Settings` :!label _label_3)))
        (else
          (goto _label_2)))
      (else
        (goto _label)))
    (else
      (goto _label_3))))

(fn `Print Array String`
  (params (Array :type "Array of EHandKeypoint Enum") (`String Start` :type String))
  (set `self.TempText` `String Start`)
  (for _array_element Array
    (bind _output_get (set `self.TempText` (`KismetStringLibrary.Concat_StrStr` (stale _output_get) "::" (`|GetEnumeratorNameAsString` _array_element)))))
  (`KismetSystemLibrary.PrintString` _output_get))

(fn `Set Damping`
  (params (`Static Mesh` :type "StaticMeshComponent Object Reference") (InDamping :type "Float (double-precision)"))
  (`/Engine/EditorBlueprintResources/StandardMacros.IsValid` `Static Mesh`
    (:`Is Valid`
      (`PrimitiveComponent.SetLinearDamping` `Static Mesh` InDamping)
      (`PrimitiveComponent.SetAngularDamping` `Static Mesh` InDamping))))

(fn `Set Default Settings`
  (bind _cube (`self.Cube`))
  (`PrimitiveComponent.SetMaterial` _cube 0 "/Game/Materials/Emissive_Material_Inst_Blue.Emissive_Material_Inst_Blue")
  (`PrimitiveComponent.SetCollisionObjectType` _cube "ECC_PhysicsBody")
  (`PrimitiveComponent.SetCollisionEnabled` _cube "QueryAndPhysics")
  (`self.Set Damping` _cube (`self.Free Damping`))
  (set `self.bCanBeDamaged` true)
  (`PrimitiveComponent.SetSimulatePhysics` _cube true)
  (return))

(fn `set Held Settings`
  (bind _cube (`self.Cube`))
  (`PrimitiveComponent.SetSimulatePhysics` _cube false)
  (`PrimitiveComponent.SetCollisionEnabled` _cube "NoCollision")
  (`PrimitiveComponent.SetCollisionObjectType` _cube "ECC_GameTraceChannel1")
  (set `self.bCanBeDamaged` false)
  (`self.Set Damping` _cube (`self.Held Damping`)))

(fn `UserConstructionScript`)