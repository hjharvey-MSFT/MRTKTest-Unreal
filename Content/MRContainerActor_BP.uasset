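; MRContainerActor_BP is an actor that runs a mixed reality AR session with tap and hold gestures and spatial mapping.
; On BeginPlay it starts the session and retries spatial mapping capture on a short timer until it succeeds; EndPlay stops both.
; ARTrackableNotify add and update events show tracked meshes with an assigned material, while hand and unclassified (NotApplicable) meshes are hidden, with hand-mesh collision disabled.
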(event `self.ReceiveBeginPlay`
  (`ARBlueprintLibrary.StartARSession` "/Game/MRSessionConfig.MRSessionConfig")
  (`HeadMountedDisplayFunctionLibrary.ConfigureGestures` (make `XRGestureConfig` true true))
  (bind _returnvalue (`ARBlueprintLibrary.IsARSupported`))
  (if _returnvalue
    (`self.EnabledSpatialMappingRecurse`)))

(event `self.ReceiveEndPlay`
  (params (EndPlayReason :type "EEndPlayReason Enum" :default "Destroyed"))
  (bind _returnvalue (`ARBlueprintLibrary.IsARSupported`))
  (if _returnvalue
    (`ARBlueprintLibrary.ToggleARCapture` false "SpatialMapping")
    (`ARBlueprintLibrary.StopARSession`)))

(event `self.ReceiveTick`
  (params (DeltaSeconds :type "Float (single-precision)")))

(event `self.ARTrackableNotify.OnAddTrackedGeometry`
  (params (TrackedGeometry :type "ARTrackedGeometry Object Reference"))
  (`self.ToggleSpatialMesh` TrackedGeometry true))

(event `self.ARTrackableNotify.OnUpdateTrackedGeometry`
  (params (TrackedGeometry :type "ARTrackedGeometry Object Reference"))
  (`self.ToggleSpatialMesh` TrackedGeometry true))

(event `self.ARTrackableNotify.OnRemoveTrackedGeometry`
  (params (TrackedGeometry :type "ARTrackedGeometry Object Reference")))

(fn `EnabledSpatialMappingRecurse`
  (bind _returnvalue (`ARBlueprintLibrary.ToggleARCapture` true "SpatialMapping"))
  ;[1 1 1] Keep enabling until it is successful.
  (if (not _returnvalue)
    (`KismetSystemLibrary.K2_SetTimer` null "EnabledSpatialMappingRecurse" 0.2)))

(fn `ToggleSpatialMesh`
  (params (Geometry :type "ARTrackedGeometry Object Reference") (IsEnabled :type Boolean))
  (bind _returnvalue (`ARTrackedGeometry.GetUnderlyingMesh` Geometry))
  (bind _returnvalue_2 (`ARTrackedGeometry.GetObjectClassification` Geometry))
  (`/Engine/EditorBlueprintResources/StandardMacros.IsValid` _returnvalue
    (:`Is Valid`
      (if (or (`|EnumEquality` _returnvalue_2 "HandMesh") (`|EnumEquality` _returnvalue_2 "NotApplicable"))
        ;[1 1 1] Hide/Disable Hand Meshes
        (`SceneComponent.SetVisibility` _returnvalue false false)
        (`PrimitiveComponent.SetCollisionEnabled` _returnvalue "NoCollision")
        (else
          (`SceneComponent.SetVisibility` _returnvalue IsEnabled false)
          (`PrimitiveComponent.SetMaterial` _returnvalue 0 (`self.Material`)))))))

(fn `UserConstructionScript`)